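; BP_Switch is an interactable light switch that toggles the point light of a referenced LightHolder when E is pressed.
; Overlapping Box enables the actor's input for player controller 0, without filtering the overlapping actor, and leaving disables it.
; Each press flips the Switch flag, which only selects which of two sounds plays alongside the visibility toggle.
; A second volume, BoxTextRender, shows the TextRender prompt only while BP_Player overlaps it.
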(event `Key|E`
  (params (Key :type "Key Structure"))
  (bind _pointlightcomponent (`PointLight.PointLightComponent` (`self.LightHolder`)))
  (:`Pressed`
    (if (`self.Switch`)
      (`GameplayStatics.PlaySound2D` "/Game/Interface_Item_Sounds_LITE/MISC/wav/Hint_1_3.Hint_1_3" 1.0 1.0 0.0 null null)
      (`SceneComponent.ToggleVisibility` _pointlightcomponent false)
      (set `self.Switch` false)
      (else
        (`GameplayStatics.PlaySound2D` "/Game/Interface_Item_Sounds_LITE/MISC/wav/Hint_1_1.Hint_1_1" 1.0 1.0 0.0 null null)
        (`SceneComponent.ToggleVisibility` _pointlightcomponent false)
        (set `self.Switch` true)))))

(event `self.Box.OnComponentBeginOverlap`
  (params (OverlappedComponent :type "PrimitiveComponent Object Reference") (OtherActor :type "Actor Object Reference") (OtherComp :type "PrimitiveComponent Object Reference") (OtherBodyIndex :type Integer) (bFromSweep :type Boolean) (SweepResult :type "HitResult Structure (by ref)"))
  (`self.EnableInput` (`GameplayStatics.GetPlayerController` 0)))

(event `self.Box.OnComponentEndOverlap`
  (params (OverlappedComponent :type "PrimitiveComponent Object Reference") (OtherActor :type "Actor Object Reference") (OtherComp :type "PrimitiveComponent Object Reference") (OtherBodyIndex :type Integer))
  (`self.DisableInput` (`GameplayStatics.GetPlayerController` 0)))

(event `self.BoxTextRender.OnComponentBeginOverlap`
  (params (OverlappedComponent :type "PrimitiveComponent Object Reference") (OtherActor :type "Actor Object Reference") (OtherComp :type "PrimitiveComponent Object Reference") (OtherBodyIndex :type Integer) (bFromSweep :type Boolean) (SweepResult :type "HitResult Structure (by ref)"))
  (cast `/Game/Blueprints/BP_Player` OtherActor)
  (`SceneComponent.SetHiddenInGame` (`self.TextRender`) false false))

(event `self.BoxTextRender.OnComponentEndOverlap`
  (params (OverlappedComponent :type "PrimitiveComponent Object Reference") (OtherActor :type "Actor Object Reference") (OtherComp :type "PrimitiveComponent Object Reference") (OtherBodyIndex :type Integer))
  (cast `/Game/Blueprints/BP_Player` OtherActor)
  (`SceneComponent.SetHiddenInGame` (`self.TextRender`) true false))

(fn `UserConstructionScript`)