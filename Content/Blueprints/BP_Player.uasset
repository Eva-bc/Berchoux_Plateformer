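; Player Blueprint that collects items and interacts with chests and a kitten.
; BeginPlay shows fish-bone and cat-food HUD widgets after a delay.
; Overlapping a collectible component passes it to the collect component and refreshes the main HUD score.
; E sends an InteractInterface message to the first overlapping chest and FeedText actor, while the Interact input action runs a sphere trace whose result is unused.
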(event `self.ReceiveBeginPlay`
  (`parent.ReceiveBeginPlay`)
  (`|ExecutionSequence`
    (:`then_0`
      ;[1 1 1] Affichage des os de poissons
      (`KismetSystemLibrary.Delay` 2.5)
      (bind _returnvalue (`|CreateWidget` "/Game/Widgets/BPW_MainHUD.BPW_MainHUD_C"))
      (`UserWidget.AddToViewport` _returnvalue 0)
      (set `self.HUD` _returnvalue))
    (:`then_1`
      ;[1 1 1] Affichage des patés pour chat
      (`KismetSystemLibrary.Delay` 2.5)
      (bind _returnvalue_2 (`|CreateWidget` "/Game/Widgets/BPW_CatFood.BPW_CatFood_C"))
      (`UserWidget.AddToViewport` _returnvalue_2 0)
      (set `self.HUDCatFood` _returnvalue_2))))

(event `self.ReceiveActorBeginOverlap`
  (params (OtherActor :type "Actor Object Reference"))
  (bind _returnvalue (`self.GetComponentByClass` OtherActor "/Game/Blueprints/BPC_CollectibleComponent.BPC_CollectibleComponent_C"))
  ;[1 1 1] Collecter et mettre à jour le score
  (`/Engine/EditorBlueprintResources/StandardMacros.IsValid` _returnvalue
    (:`Is Valid`
      (`/Game/Blueprints/BPC_CollectComponent.Collect` (`self.BPC_CollectComponent`) _returnvalue)
      (`/Game/Widgets/BPW_MainHUD.Update Score` (`self.HUD`)))))

(event `EnhancedInput|/Game/ThirdPerson/Input/Actions/NewInputAction_Interact`
  (params (ActionValue :type Boolean) (ElapsedSeconds :type "Float (double-precision)") (TriggeredSeconds :type "Float (double-precision)") (InputAction :type "InputAction Object Reference" :default "/Game/ThirdPerson/Input/Actions/NewInputAction_Interact.NewInputAction_Interact"))
  (:`Triggered`
    (`KismetSystemLibrary.SphereTraceMulti` (`self.K2_GetActorLocation`) (0.0 0.0 0.0) 0.0 "TraceTypeQuery1")))

(event `Key|E`
  (params (Key :type "Key Structure"))
  ;[1 1 1] Interaction du coffre
  (:`Pressed`
    (for _array_element (`self.GetOverlappingActors` "/Game/Blueprints/BP_Chest.BP_Chest_C")
      (if (`KismetSystemLibrary.DoesImplementInterface` _array_element "/Game/Blueprints/InteractInterface.InteractInterface_C")
        (message `/Game/Blueprints/InteractInterface.InteractWithChest` _array_element)
        (break)))
    ;[1 1 1] Interaction avec le bébé chat
    (for _array_element_2 (`self.GetOverlappingActors` "/Game/Blueprints/FeedText.FeedText_C")
      (if (`KismetSystemLibrary.DoesImplementInterface` _array_element_2 "/Game/Blueprints/InteractInterface.InteractInterface_C")
        (message `/Game/Blueprints/InteractInterface.InteractWithChest` _array_element_2)
        (break)))))

(fn `UserConstructionScript`
  (`parent.UserConstructionScript`))