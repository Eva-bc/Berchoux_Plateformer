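; BP_SwitchLevl2 is an interactable switch, named for level 2, that toggles the shared Switch flag in BP_GameInstance when E is pressed.
; Each toggle plays one of two hint sounds depending on the new state.
; Box overlaps enable and disable input from player controller 0 without checking which actor overlaps.
; A separate BoxTextRender volume shows the TextRender while BP_Player is inside.
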(event `self.ReceiveBeginPlay`
  (bind _asbp_game_instance (cast `/Game/Blueprints/BP_GameInstance` (`GameplayStatics.GetGameInstance`)))
  (set `self.BP Game Instance` _asbp_game_instance))

(event `Key|E`
  (params (Key :type "Key Structure"))
  (:`Pressed`
    (if (`/Game/Blueprints/BP_GameInstance.Switch` (`self.BP Game Instance`))
      (`GameplayStatics.PlaySound2D` "/Game/Interface_Item_Sounds_LITE/MISC/wav/Hint_1_3.Hint_1_3" 1.0 1.0 0.0 null null)
      (set `/Game/Blueprints/BP_GameInstance.Switch` false (`self.BP Game Instance`))
      (else
        (`GameplayStatics.PlaySound2D` "/Game/Interface_Item_Sounds_LITE/MISC/wav/Hint_1_1.Hint_1_1" 1.0 1.0 0.0 null null)
        (set `/Game/Blueprints/BP_GameInstance.Switch` true (`self.BP Game Instance`))))))

(event `self.Box.OnComponentBeginOverlap`
  (params (OverlappedComponent :type "PrimitiveComponent Object Reference") (OtherActor :type "Actor Object Reference") (OtherComp :type "PrimitiveComponent Object Reference") (OtherBodyIndex :type Integer) (bFromSweep :type Boolean) (SweepResult :type "HitResult Structure (by ref)"))
  (`self.EnableInput` (`GameplayStatics.GetPlayerController` 0)))

(event `self.Box.OnComponentEndOverlap`
  (params (OverlappedComponent :type "PrimitiveComponent Object Reference") (OtherActor :type "Actor Object Reference") (OtherComp :type "PrimitiveComponent Object Reference") (OtherBodyIndex :type Integer))
  (`self.DisableInput` (`GameplayStatics.GetPlayerController` 0)))

(event `self.BoxTextRender.OnComponentBeginOverlap`
  (params (OverlappedComponent :type "PrimitiveComponent Object Reference") (OtherActor :type "Actor Object Reference") (OtherComp :type "PrimitiveComponent Object Reference") (OtherBodyIndex :type Integer) (bFromSweep :type Boolean) (SweepResult :type "HitResult Structure (by ref)"))
  (cast `/Game/Blueprints/BP_Player` OtherActor)
  (`SceneComponent.SetHiddenInGame` (`self.TextRender`) false false))

(event `self.BoxTextRender.OnComponentEndOverlap`
  (params (OverlappedComponent :type "PrimitiveComponent Object Reference") (OtherActor :type "Actor Object Reference") (OtherComp :type "PrimitiveComponent Object Reference") (OtherBodyIndex :type Integer))
  (cast `/Game/Blueprints/BP_Player` OtherActor)
  (`SceneComponent.SetHiddenInGame` (`self.TextRender`) true false))

(fn `UserConstructionScript`)