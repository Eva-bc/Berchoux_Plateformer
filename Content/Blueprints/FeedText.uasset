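; FeedText is an interactable actor that shows a world-space text prompt and ends the game once enough special items (cat pâté) are collected.
; Its Box overlap events show the TextRender when BP_Player enters and hide it on exit.
; InteractwithChest checks SpecialScore on the Game Instance cached at BeginPlay.
; If the threshold is met, it displays the BPW_End widget and quits after a short delay.
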(event `self.ReceiveBeginPlay`
  ;[1 1 1] Faire appelle au Game Instance
  (bind _asbp_game_instance (cast `/Game/Blueprints/BP_GameInstance` (`GameplayStatics.GetGameInstance`)))
  (set `self.BP Game Instance` _asbp_game_instance))

(event `self.Box.OnComponentBeginOverlap`
  (params (OverlappedComponent :type "PrimitiveComponent Object Reference") (OtherActor :type "Actor Object Reference") (OtherComp :type "PrimitiveComponent Object Reference") (OtherBodyIndex :type Integer) (bFromSweep :type Boolean) (SweepResult :type "HitResult Structure (by ref)"))
  ;[1 1 1] Afficher le texte
  (cast `/Game/Blueprints/BP_Player` OtherActor)
  (`SceneComponent.SetHiddenInGame` (`self.TextRender`) false false))

(event `self.Box.OnComponentEndOverlap`
  (params (OverlappedComponent :type "PrimitiveComponent Object Reference") (OtherActor :type "Actor Object Reference") (OtherComp :type "PrimitiveComponent Object Reference") (OtherBodyIndex :type Integer))
  ;[1 1 1] Afficher le texte
  (cast `/Game/Blueprints/BP_Player` OtherActor)
  (`SceneComponent.SetHiddenInGame` (`self.TextRender`) true false))

(event `/Game/Blueprints/InteractInterface.InteractWithChest`
  ;[1 1 1] Si il y a assez de paté pour chat le jeu s'arrete
  (if (>= (`/Game/Blueprints/BP_GameInstance.SpecialScore` (`self.BP Game Instance`)) 3)
    (bind _returnvalue (`|CreateWidget` "/Game/Widgets/BPW_End.BPW_End_C"))
    (`UserWidget.AddToViewport` _returnvalue 0)
    (`KismetSystemLibrary.Delay` 2.5)
    (`KismetSystemLibrary.QuitGame` null "Quit")))

(fn `UserConstructionScript`)