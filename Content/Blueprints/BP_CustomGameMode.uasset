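; BP_CustomGameMode is a game mode that runs a one-time player position fix when play begins.
; On BeginPlay it casts to BP_GameInstance and, if its LazyFix flag is unset, teleport-free moves the player pawn to a hard-coded location and sets the flag.
; Because the flag lives on the game instance, the move happens only once per session, not on later level loads.
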(event `self.ReceiveBeginPlay`
  (bind _asbp_game_instance (cast `/Game/Blueprints/BP_GameInstance` (`GameplayStatics.GetGameInstance`)))
  (set `self.As BP Game Instance` _asbp_game_instance)
  (if (not (`/Game/Blueprints/BP_GameInstance.LazyFix` (`self.As BP Game Instance`)))
    (`self.K2_SetActorLocation` (`GameplayStatics.GetPlayerPawn` 0) (810.0 1110.0 92.012604) false false)
    (set `/Game/Blueprints/BP_GameInstance.LazyFix` true (`self.As BP Game Instance`))))

(event `self.ReceiveTick`
  (params (DeltaSeconds :type "Float (single-precision)")))

(fn `UserConstructionScript`
  (`parent.UserConstructionScript`))