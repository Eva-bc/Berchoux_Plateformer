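; BPC_CollectComponent is a component that collects pickups and adds their value to scores on the game instance.
; It caches BP_GameInstance at BeginPlay, so Collect writes directly to that shared object.
; Collect branches on the collectible's IsSpecial flag: cat pâté adds to SpecialScore and fish bones to Score, each with its own 2D sound.
; It then calls DestroyBPComponent on the collectible.
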(event `self.ReceiveBeginPlay`
  (bind _asbp_game_instance (cast `/Game/Blueprints/BP_GameInstance` (`GameplayStatics.GetGameInstance`)))
  (set `self.BP Game Instance` _asbp_game_instance))

(fn `Collect`
  (params (Collectible :type "/Game/Blueprints/BPC_CollectibleComponent Object Reference"))
  (bind _bp_game_instance (`self.BP Game Instance`))
  ;[1 1 1] Vérifier si l'objet collecter est bien de la paté pour chat
  (if (`/Game/Blueprints/BPC_CollectibleComponent.IsSpecial` Collectible)
    ;[1 1 1] Collecter et rajouter le score de mes patés pour chat
    (set `/Game/Blueprints/BP_GameInstance.SpecialScore` (+ (`/Game/Blueprints/BPC_CollectibleComponent.SpecialScoreValue` Collectible) (`/Game/Blueprints/BP_GameInstance.SpecialScore` _bp_game_instance)) _bp_game_instance)
    (`GameplayStatics.PlaySound2D` "/Game/Interface_Item_Sounds_LITE/Items_Collectibles/wav/Coin_3_3.Coin_3_3" 1.0 1.0 0.0 null null)
    (else
      ;[1 1 1] Collecter et rajouter le score de mes os de poissons
      (set `/Game/Blueprints/BP_GameInstance.Score` (+ (`/Game/Blueprints/BPC_CollectibleComponent.Value` Collectible) (`/Game/Blueprints/BP_GameInstance.Score` _bp_game_instance)) _bp_game_instance)
      (`GameplayStatics.PlaySound2D` "/Game/Interface_Item_Sounds_LITE/Interface/cue/Bubble_02_Cue.Bubble_02_Cue" 1.0 1.0 0.0 null null)))
  (`/Game/Blueprints/BPC_CollectibleComponent.DestroyBPComponent` Collectible))