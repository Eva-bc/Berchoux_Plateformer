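; BP_Chest is an interactable chest that plays an open/close animation and spawns an item, apparently cat food.
; InteractwithChest plays the animation on every call, while a DoOnce limits the spawn to the first one.
; Spawn creates the SpawnCatFood class at the BoxSpawn location, ignoring collisions.
; Box overlaps show or hide the TextRender prompt when BP_Player enters or leaves.
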(event `/Game/Blueprints/BPI_InteractInterface.InteractWithChest`
  ;[1 1 1] Animation du coffre
  (`SkeletalMeshComponent.PlayAnimation` (`self.SkeletalMesh`) "/Game/low-poly-chest-animated/source/Chest_Animated_Anim_Chest_Up_Chest_Open_Close.Chest_Animated_Anim_Chest_Up_Chest_Open_Close" false)
  ;[1 1 1] "Spwan" une seule fois l'objet du coffre
  (`/Engine/EditorBlueprintResources/StandardMacros.DoOnce` false
    (:`Completed`
      (`self.Spawn`))))

(event `self.Box.OnComponentBeginOverlap`
  (params (OverlappedComponent :type "PrimitiveComponent Object Reference") (OtherActor :type "Actor Object Reference") (OtherComp :type "PrimitiveComponent Object Reference") (OtherBodyIndex :type Integer) (bFromSweep :type Boolean) (SweepResult :type "HitResult Structure (by ref)"))
  ;[1 1 1] Afficher et cacher le texte du coffre
  (cast `/Game/Blueprints/BP_Player` OtherActor)
  (`SceneComponent.SetHiddenInGame` (`self.TextRender`) false false))

(event `self.Box.OnComponentEndOverlap`
  (params (OverlappedComponent :type "PrimitiveComponent Object Reference") (OtherActor :type "Actor Object Reference") (OtherComp :type "PrimitiveComponent Object Reference") (OtherBodyIndex :type Integer))
  ;[1 1 1] Afficher et cacher le texte du coffre
  (cast `/Game/Blueprints/BP_Player` OtherActor)
  (`SceneComponent.SetHiddenInGame` (`self.TextRender`) true false))

(event `Spawn`
  ;[1 1 1] Faire "spawn" un objet du coffre
  (`|SpawnActorFromClass` (`self.SpawnCatFood`) (`KismetMathLibrary.MakeTransform` (`SceneComponent.K2_GetComponentLocation` (`self.BoxSpawn`))) "AlwaysSpawn" "MultiplyWithRoot" null null))

(fn `UserConstructionScript`)